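; Tank pawn Blueprint that the player drives, aims and fires, with a health bar widget linked to it.
; BeginPlay hands barrel, turret and track references to the TankAiming and TankMovement components and sets itself as the health bar's tank.
; Axis inputs throttle each track forward or backward independently and rotate an azimuth gimbal and spring arm to orbit the camera.
; Fire calls TankAiming, and SwapCamera toggles first- and third-person cameras.
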(event `self.ReceiveBeginPlay`
  (`TankAimingComponent.Initialize` (`self.TankAiming`) (`self.TankBarrel`) (`self.TankTurrent`))
  (`TankMovementComponent.Initialize` (`self.TankMovement`) (`self.LeftTrack`) (`self.RightTrack`))
  (`self.InitializeHealthBarFunction`))

(event `InputAction|SwapCamera`
  (params (Key :type "Key Structure"))
  (:`Pressed`
    (`ActorComponent.ToggleActive` (`self.3rd person camera`))
    (`ActorComponent.ToggleActive` (`self.1st person camera`))))

(event `InputAxis|LeftTrackForward`
  (params (AxisValue :type "Float (single-precision)"))
  ;[1 1 1] Movement
  (`TankMovementComponent.AddThrottleToTrack` (`self.TankMovement`) (`self.LeftTrack`) AxisValue))

(event `InputAxis|AimElevation`
  (params (AxisValue :type "Float (single-precision)"))
  ;[1 1 1] Camera input binding
  (`SceneComponent.K2_AddLocalRotation` (`self.SpringArm`) (`KismetMathLibrary.MakeRotator` 0.0 (* AxisValue (`GameplayStatics.GetWorldDeltaSeconds`) 150.0)) false false))

(event `InputAxis|RightTrackForward`
  (params (AxisValue :type "Float (single-precision)"))
  ;[1 1 1] Movement
  (`TankMovementComponent.AddThrottleToTrack` (`self.TankMovement`) (`self.RightTrack`) AxisValue))

(event `InputAxis|AimAzimuth`
  (params (AxisValue :type "Float (single-precision)"))
  ;[1 1 1] Camera input binding
  (`SceneComponent.K2_AddLocalRotation` (`self.AzimuthGimbal`) (`KismetMathLibrary.MakeRotator` 0.0 0.0 (* AxisValue (`GameplayStatics.GetWorldDeltaSeconds`) 150.0)) false false))

(event `InputAxis|LeftTrackBackward`
  (params (AxisValue :type "Float (single-precision)"))
  ;[1 1 1] Movement
  (`TankMovementComponent.AddThrottleToTrack` (`self.TankMovement`) (`self.LeftTrack`) (* -1 AxisValue)))

(event `InputAction|Fire`
  (params (Key :type "Key Structure"))
  ;[1 1 1] Fire input binding
  (:`Pressed`
    (`TankAimingComponent.Fire` (`self.TankAiming`))))

(event `InputAxis|RightTrackBackward`
  (params (AxisValue :type "Float (single-precision)"))
  ;[1 1 1] Movement
  (`TankMovementComponent.AddThrottleToTrack` (`self.TankMovement`) (`self.RightTrack`) (* -1 AxisValue)))

(fn `InitializeHealthBarFunction`
  (bind _ashealth_bar (cast `/Game/Ui/HealthBar` (`WidgetComponent.GetUserWidgetObject` (`self.HealthBar`))))
  (set `/Game/Ui/HealthBar.MyTank` self _ashealth_bar)
  (return))

(fn `UserConstructionScript`)